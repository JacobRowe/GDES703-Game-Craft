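; EnemSpawner_BP is an enemy spawner that produces waves of enemies from BeginPlay onward.
; Each wave loops over NoOfEnemies, spawning the Enemy class at the spawner's transform plus a separate, hard-coded Enemy_Imp running ImpAI_BT, with no location set.
; SpawnEnemy then waits SpawnDelay and calls itself again, so waves repeat with no stop condition.
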(event Custom|Spawn%20Enemy
  (params (Enemy :type Actor%20Class%20Reference) (SpawnTransform :type Transform) (No%20Of%20Enemies :type Integer))
  (for _index (range 0 (- No%20Of%20Enemies 1))
    (Game|SpawnActorfromClass Enemy SpawnTransform "Undefined" 0 0)
    (AI|SpawnAIFromClass "/Game/Enemy/Imp/Enemy_Imp.Enemy_Imp_C" "/Game/Enemy/Imp/ImpAI_BT.ImpAI_BT" "0, 0, 0" "0, 0, 0" false 0))
  (Utilities|FlowControl|Delay (Variables|Default|GetSpawn%20Delay))
  (CallFunction|SpawnEnemy (Variables|Default|GetEnemy) (Transformation|GetActorTransform) (Variables|Default|GetNo%20Of%20Enemies)))

(event EventBeginPlay
  (CallFunction|SpawnEnemy (Variables|Default|GetEnemy) (Transformation|GetActorTransform) (Variables|Default|GetNo%20Of%20Enemies)))

(fn ConstructionScript)