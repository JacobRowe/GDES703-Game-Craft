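; EnemyAreaSpawn_BP is an area spawner meant to create enemies at random points inside its SpawnArea bounds.
; On BeginPlay it sets a looping timer for Spawn Enemy on the first spawner found in the world, using EnemiesPerSecond as the interval.
; The event checks the Enemy_Imp count against MaxEnemies, but the branch leads nowhere.
; The SpawnAIFromClass call is disconnected, so nothing spawns.
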(event Custom|Spawn%20Enemy
  (bind _outactors (Actor|GetAllActorsOfClass "/Game/Enemy/Imp/Enemy_Imp.Enemy_Imp_C"))
  (if (<= (Utilities|Array|Length _outactors) (Variables|Default|GetMax%20Enemies))
    _))

(event EventBeginPlay
  (bind _outactors (Actor|GetAllActorsOfClass "EnemyAreaSpawn_BP_C"))
  (bind _output_get (Variables|Default|SetSpawner (Utilities|Array|Get(acopy) _outactors)))
  (Utilities|Time|SetTimerbyFunctionName _output_get "Spawn Enemy" (Variables|Default|GetEnemies%20Per%20Second) true))

(fn ConstructionScript)